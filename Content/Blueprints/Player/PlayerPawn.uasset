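; Player pawn for a card game that switches its camera between preset viewpoints and draws cards into the hand.
; Space toggles between two viewpoints, with a timeline blending the camera's relative transform toward targets looked up in a Positions map keyed by viewpoint enum.
; E draws a card from the BP_Deck actor and adds it to BP_Hand, both found by class lookup.
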(event Custom|SetViewpoint
  (params (viewpoint :type EPlayerViewpoint%20Enum :default "NewEnumerator0"))
  (bind _camera (Variables|Default|GetCamera))
  (bind _positions (Variables|Default|Getpositions))
  (bind _returnvalue (Transformation|GetRelativeTransform _camera))
  (bind _value (Utilities|Map|Find _positions viewpoint))
  (bind _alpha (Timeline|LerpToViewpoint PlayFromStart)
    (:Update
      (Transformation|SetRelativeLocationAndRotation (Variables|Default|GetCamera) (Math|Vector|Lerp(Vector) (.location _returnvalue) (.location _value) _alpha) (Math|Rotator|Lerp(Rotator) (.rotation _returnvalue) (.rotation _value) _alpha true) false true))))

(event EventBeginPlay
  (Input|EnableInput (Game|GetPlayerController 0))
  (CallFunction|SetViewpoint "NewEnumerator0"))

(event Input|KeyboardEvents|SpaceBar
  (params (Key :type Key%20Structure :default "None"))
  (:Pressed
    (Utilities|FlowControl|FlipFlop
      (:A
        (CallFunction|SetViewpoint "NewEnumerator1"))
      (:B
        (CallFunction|SetViewpoint "NewEnumerator0")))))

(event Input|KeyboardEvents|E
  (params (Key :type Key%20Structure :default "None"))
  (:Pressed
    (bind _returnvalue (Actor|GetActorOfClass "/Game/Blueprints/Cards/Decks/BP_Deck.BP_Deck_C"))
    (bind _card (Default|Draw _returnvalue))
    (bind _returnvalue_2 (Actor|GetActorOfClass "/Game/Blueprints/Cards/BP_Hand.BP_Hand_C"))
    (Default|AddCard _returnvalue_2 _card)))

(fn ConstructionScript)