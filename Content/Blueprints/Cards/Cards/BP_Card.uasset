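; BP_Card is a card Blueprint that shows its card data through a W_Card widget.
; On BeginPlay, if the GetDataFromName variable is not "None", it looks up card data by that name and replaces its CardData when the lookup succeeds.
; It then calls UpdateData, which stores the data and passes it to the widget's UpdateCardInfo.
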(event EventBeginPlay
  (bind _getdatafromname (Variables|Default|GetgetDataFromName))
  (bind (_carddata _success) (CallFunction|GetCardDatabyName _getdatafromname))
  (Utilities|FlowControl|Sequence
    (:then_0
      (if (!= (Variables|Default|GetgetDataFromName) "None")
        (if _success
          (Variables|Default|SetcardData _carddata))))
    (:then_1
      (CallFunction|UpdateData (Variables|Default|GetcardData)))))

(fn ConstructionScript)

(fn UpdateData
  (params (cardData :type S%20Card%20Data%20Structure))
  (bind _output_get (Variables|Default|SetcardData cardData))
  (Default|UpdateCardInfo (.AsW%20Card (Utilities|Casting|CastToW_Card (UserInterface|GetUserWidgetObject (Variables|Default|GetWidget)))) _output_get))