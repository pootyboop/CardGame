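; BP_Deck is a card deck that holds an ordered list of card names and hands out cards drawn from the top.
; On BeginPlay it optionally replaces DeckData with a small hardcoded default deck, then copies the data's card list into the working Deck array.
; Draw creates a card from the first name, removing that entry only if creation succeeds, with no empty-deck check or shuffling.
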(event EventBeginPlay
  (Utilities|FlowControl|Sequence
    (:then_0
      (if (Variables|Default|GetuseDefaultDeck)
        (Variables|Default|SetdeckData (Utilities|Struct|MakeSDeck (Utilities|Array|MakeArray "Gudditi" "Slikit Adolescent" "Gudditi" "Slikit Adolescent")))))
    (:then_1
      (Variables|Default|Setdeck (Utilities|Struct|BreakSDeck (Variables|Default|GetdeckData))))))

(fn ConstructionScript)

(fn Draw
  (bind _output_get (LocalVariables|SetdrawnCard (Utilities|Array|Get(acopy) (Variables|Default|Getdeck))))
  (bind (_card _success) (CallFunction|CreateCardbyName :cardName _output_get))
  (if _success
    (Utilities|Array|RemoveIndex (Variables|Default|Getdeck))
    (return _card true)
    (else
      (return 0 false))))