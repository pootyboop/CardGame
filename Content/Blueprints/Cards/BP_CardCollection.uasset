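; BP_CardCollection is an actor that holds a collection of cards and shows each one on its own BP_CardSpace.
; AddCard appends to the Cards array and calls ResizeCollection, which clears and destroys all existing spaces, then rebuilds them from scratch.
; Each new space takes the collection's type, snaps to the collection actor and receives its card.
; The rebuild appends to Spaces without emptying the array.
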(event EventBeginPlay)

(fn ConstructionScript)

(fn AddCard
  (params (card :type BP%20Card%20Object%20Reference))
  (Utilities|Array|Add (Variables|Default|Getcards) card)
  (CallFunction|ResizeCollection))

(fn ResizeCollection
  (Utilities|FlowControl|Sequence
    (:then_0
      (for _array_element (Variables|Default|Getspaces)
        (Default|ClearSpace _array_element)
        (Actor|DestroyActor _array_element)))
    (:then_1
      (for _array_element_2 (Variables|Default|Getcards)
        (bind _returnvalue (Game|SpawnActorfromClass "/Game/Blueprints/PlayArea/CardSpaces/BP_CardSpace.BP_CardSpace_C" (Math|Transform|MakeTransform "0, 0, 0") "Undefined" "MultiplyWithRoot" 0 (Utilities|Struct|MakeSCardSpaceInfo (Variables|Default|GetcollectionType) "(width_5_ED483AFA4F94F53A906806903FB21856=5,height_6_2A1C03A54B5C315503B594A8DCD8632F=6)") "(R=0.126298,G=0.146374,B=0.312500,A=1.000000)" 0))
        (Transformation|AttachActorToActor _returnvalue self "None" "SnapToTarget" "SnapToTarget" "SnapToTarget" true)
        (Utilities|Array|Add (Variables|Default|Getspaces) _returnvalue)
        (Default|PlaceCard _returnvalue _array_element_2)))))