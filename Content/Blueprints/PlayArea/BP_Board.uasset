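; BP_Board is the card game's play area, spawning a grid of BP_CardSpace actors on BeginPlay.
; InitBoard loops over the board width on both axes, passing each space its grid position and giving both edge rows along the second axis a distinct type.
; Transforms derive from card dimensions plus a margin, with spaces rotated 180 degrees when the first player controller has authority.
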(event EventBeginPlay
  (CallFunction|InitBoard))

(fn ConstructionScript)

(fn InitBoard
  (bind _boardsize (CallFunction|GetBoardSize))
  (bind _width (Utilities|Struct|BreakSBoardSize _boardsize))
  (bind _returnvalue (- _width 1))
  (for _index (range 0 (- _width 1))
    (for _index_2 (range 0 _returnvalue)
      (Game|SpawnActorfromClass "/Game/Blueprints/PlayArea/CardSpaces/BP_CardSpace.BP_CardSpace_C" (CallFunction|SolveNewBoardCardSpaceTransform (Utilities|Struct|MakeSBoardSize _index _index_2)) "Undefined" "MultiplyWithRoot" 0 (Utilities|Struct|MakeSCardSpaceInfo (select (or (== _index_2 0) (== _index_2 _returnvalue)) "NewEnumerator3" "NewEnumerator0") (Utilities|Struct|MakeSBoardSize _index _index_2)) "(R=0.312500,G=0.312500,B=0.312500,A=1.000000)" 0))))

(fn SolveNewBoardCardSpaceTransform
  (params (boardPos :type S%20Board%20Size%20Structure))
  (bind (_width _height) (Utilities|Struct|BreakSBoardSize boardPos))
  (bind _carddimensions (CallFunction|GetCardDimensions))
  (bind _returnvalue (Class|KismetSystemLibrary|MakeLiteralInteger 100))
  (bind (_x _y) (Math|Vector2D|BreakVector2D _carddimensions))
  (return (Math|Transform|MakeTransform (Math|Vector|MakeVector (CallFunction|ApplyBoardCardSpaceMargin (* _width _returnvalue _x) _width) (CallFunction|ApplyBoardCardSpaceMargin (* _height _returnvalue _y) _height) 0.0) (select (Ability|HasAuthority (Game|GetPlayerController 0)) "0.000000,180.000000,0.000000" "0, 0, 0"))))

(fn ApplyBoardCardSpaceMargin
  (params (actualPosition :type Integer) (boardPosition :type Integer))
  (return (+ actualPosition (* boardPosition (Variables|Default|GetcardSpaceMargin)))))