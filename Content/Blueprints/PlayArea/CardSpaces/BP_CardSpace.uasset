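; BP_CardSpace is a play-area slot that holds a single card.
; On BeginPlay it scales to card dimensions and gives its plane a dynamic material, whose Tint defaults to a stored color, or dark red for one space type.
; PlaceCard only acts on an empty space, linking card and space to each other and teleporting the card just above it.
; ClearSpace drops the space's card reference.
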(event EventBeginPlay
  (bind _carddimensions (CallFunction|GetCardDimensions))
  (bind (_x _y) (Math|Vector2D|BreakVector2D _carddimensions))
  (Transformation|SetActorScale3D (Math|Vector|MakeVector _x _y 1.0))
  (bind _returnvalue (Rendering|Material|CreateDynamicMaterialInstance "/Game/Materials/M_Master.M_Master" "None" "None" :!class /Script/Engine.KismetMaterialLibrary))
  (bind _output_get (Variables|Default|Setmat _returnvalue))
  (Rendering|Material|SetMaterial (Variables|Default|GetPlane) 0 _output_get)
  (CallFunction|RestoreDefaultColor))

(fn ConstructionScript)

(fn RestoreDefaultColor
  (CallFunction|SetColor (Math|Color|SelectColor "(R=0.333333,G=0.061111,B=0.061111,A=1.000000)" (Variables|Default|GetdefaultColor) (Utilities|Enum|Equal(Enum) (.type (Variables|Default|GetspaceInfo)) "NewEnumerator3"))))

(fn SetColor
  (params (Value :type Linear%20Color%20Structure :default "(R=1.000000,G=1.000000,B=1.000000,A=1.000000)"))
  (Rendering|Material|SetVectorParameterValue (Variables|Default|Getmat) "Tint" Value :!class /Script/Engine.MaterialInstanceDynamic))

(fn PlaceCard
  (params (card :type BP%20Card%20Object%20Reference))
  (bind _returnvalue (Transformation|GetActorTransform))
  (bind (_x _y _z) (Class|KismetMathLibrary|BreakVector3f (.location _returnvalue)))
  (if (not (CallFunction|IsOccupied))
    (bind _output_get (Variables|Default|Setcard card))
    (Variables|/Game/Blueprints/Cards/Cards/BP_Card.BP_Card_C|SetcurrSpace _output_get self)
    (Utilities|IsValid _output_get
      (:Is%20Valid
        (Transformation|SetActorTransform _output_get (Math|Transform|MakeTransform (Math|Vector|MakeVector _x _y (+ _z 1.0)) (.rotation _returnvalue)) false true)))))

(fn IsOccupied
  (return (Utilities|IsValid (Variables|Default|Getcard))))

(fn ClearSpace
  (Variables|Default|Setcard 0))