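; BPFN is a helper function library for a card game, giving shared access to the game mode and to card creation.
; It casts the current game mode to GM to expose board size and card dimensions and to delegate card spawning.
; Creation by name linearly searches DT_Cards rows on their Name field rather than the row name, returning a success flag.
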(fn GetGM
  (return (.AsGM (Utilities|Casting|CastToGM (Game|GetGameMode (LocalVariables|Get__WorldContext))))))

(fn GetBoardSize
  (return (Variables|/Game/Blueprints/GM.GM_C|GetboardSize (CallFunction|GetGM))))

(fn GetCardDimensions
  (return (Variables|/Game/Blueprints/GM.GM_C|GetcardDimensions (CallFunction|GetGM))))

(fn CreateCard
  (params (spawnTransform :type Transform) (cardData :type S%20Card%20Data%20Structure))
  (bind _card (Default|CreateCard (CallFunction|GetGM) spawnTransform cardData))
  (return _card))

(fn CreateCardbyName
  (params (spawnTransform :type Transform) (cardName :type Name))
  (bind (_carddata _success) (CallFunction|GetCardDatabyName cardName))
  (if _success
    (bind _card (CallFunction|CreateCard spawnTransform _carddata))
    (return _card true)
    (else
      (return false 0))))

(fn GetCardDatabyName
  (params (cardName :type Name))
  (bind _outrownames (DataTable|GetDataTableRowNames "/Game/Blueprints/Cards/Cards/DT_Cards.DT_Cards"))
  (for _array_element _outrownames
    (bind _returnvalue (Utilities|GetDataTableRow "/Game/Blueprints/Cards/Cards/DT_Cards.DT_Cards" _array_element)
      (:then
        (if (== (.name (Utilities|Struct|BreakSCardData _returnvalue)) cardName)
          (return _returnvalue true)))))
  (return "" false))